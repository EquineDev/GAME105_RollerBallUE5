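; BP_Ball is a player-controlled rolling ball that moves and jumps through physics impulses on its Sphere component.
; Look inputs turn the controller, and movement inputs push the sphere along control-yaw forward and right vectors, with roll also feeding the right vector.
; Jump adds an upward velocity-change impulse only when GroundCheck passes, using a debug-drawn downward line trace just past the sphere's radius.
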(event EventBeginPlay)

(event Collision|EventActorBeginOverlap
  (params (OtherActor :type Actor%20Object%20Reference)))

(event EventTick
  (params (DeltaSeconds :type Float%20%28single-precision%29)))

(event EventLookPitch
  (params (Value :type Float%20%28double-precision%29))
  ;[1 1 1] Look Camera
  (Pawn|Input|AddControllerPitchInput Value))

(event EventLookYaw
  (params (Value :type Float%20%28double-precision%29))
  ;[1 1 1] Look Camera
  (Pawn|Input|AddControllerYawInput Value))

(event EventMoveRight
  (params (Value :type Float%20%28double-precision%29))
  (bind _returnvalue (Pawn|GetControlRotation :!class /Script/Engine.Pawn))
  ;[1 1 1] Rolling
  (Physics|AddImpulse (Variables|Default|GetSphere) (* Value (Math|Vector|GetRightVector (Math|Rotator|MakeRotator (.roll _returnvalue) 0.0 (.yaw _returnvalue))) (Variables|Default|GetForce)) "None" true))

(event EventMoveFoward
  (params (Value :type Float%20%28double-precision%29))
  ;[1 1 1] Rolling
  (Physics|AddImpulse (Variables|Default|GetSphere) (* Value (Math|Vector|GetForwardVector (Math|Rotator|MakeRotator 0.0 0.0 (.yaw (Pawn|GetControlRotation :!class /Script/Engine.Pawn)))) (Variables|Default|GetForce)) "None" true))

(event EventJump
  ;[1 1 1] Jumping
  (bind _grounded (CallFunction|GroundCheck))
  (if _grounded
    (Physics|AddImpulse (Variables|Default|GetSphere) (* (Math|Vector|GetUpVector (Math|Rotator|MakeRotator 0.0 0.0 (.yaw (Pawn|GetControlRotation :!class /Script/Engine.Pawn)))) (Variables|Default|GetJumpForce)) "None" true)))

(fn ConstructionScript)

(fn GroundCheck
  (bind _returnvalue (Collision|LineTraceByChannel (Transformation|GetActorLocation) (- (Transformation|GetActorLocation) (Math|Vector|MakeVector 0.0 0.0 (+ (Class|SphereComponent|GetUnscaledSphereRadius (Variables|Default|GetSphere)) 5.0))) "TraceTypeQuery1" false 0 "ForDuration"))
  (return _returnvalue))